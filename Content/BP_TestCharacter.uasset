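; BP_TestCharacter is a test player character with a spring-arm camera that can switch shoulders.
; BeginPlay adds an Enhanced Input mapping context and puts a crosshair widget on screen.
; Input actions drive actor-relative movement, yaw and pitch look, and hold-to-crouch.
; The shoulder input flip-flops a target Y offset, which Tick smoothly interpolates into the spring arm's socket offset.
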(event Input|EnhancedActionEvents|EnhancedInputActionMove
  (params (ActionValue :type Vector%202D%20Structure) (ElapsedSeconds :type Float%20%28double-precision%29) (TriggeredSeconds :type Float%20%28double-precision%29) (InputAction :type Input%20Action%20Object%20Reference :default "/Game/Move.Move"))
  (bind (_x _y) (Math|Vector2D|BreakVector2D ActionValue))
  (Pawn|Input|AddMovementInput (Transformation|GetActorForwardVector) _y false)
  (Pawn|Input|AddMovementInput (Transformation|GetActorRightVector) _x false))

(event Input|EnhancedActionEvents|EnhancedInputActionCrouch
  (params (ActionValue :type Boolean) (ElapsedSeconds :type Float%20%28double-precision%29) (TriggeredSeconds :type Float%20%28double-precision%29) (InputAction :type Input%20Action%20Object%20Reference :default "/Game/Crouch.Crouch"))
  (:Started
    (Development|PrintString "Crouch Pressed")
    (Character|Crouch))
  (:Completed
    (Character|UnCrouch)))

(event Input|EnhancedActionEvents|EnhancedInputActionSwitch_Shoulder
  (params (ActionValue :type Boolean) (ElapsedSeconds :type Float%20%28double-precision%29) (TriggeredSeconds :type Float%20%28double-precision%29) (InputAction :type Input%20Action%20Object%20Reference :default "/Game/Switch_Shoulder.Switch_Shoulder"))
  (:Started
    (Utilities|FlowControl|FlipFlop
      (:A
        (Variables|Default|SetShoulderY 6e+01))
      (:B
        (Variables|Default|SetShoulderY -6e+01)))))

(event Input|EnhancedActionEvents|EnhancedInputActionLookx
  (params (ActionValue :type Float%20%28double-precision%29) (ElapsedSeconds :type Float%20%28double-precision%29) (TriggeredSeconds :type Float%20%28double-precision%29) (InputAction :type Input%20Action%20Object%20Reference :default "/Game/Lookx.Lookx"))
  (Pawn|Input|AddControllerYawInput ActionValue))

(event Input|EnhancedActionEvents|EnhancedInputActionLooky
  (params (ActionValue :type Float%20%28double-precision%29) (ElapsedSeconds :type Float%20%28double-precision%29) (TriggeredSeconds :type Float%20%28double-precision%29) (InputAction :type Input%20Action%20Object%20Reference :default "/Game/Looky.Looky"))
  (Pawn|Input|AddControllerPitchInput ActionValue))

(event EventBeginPlay
  (bind _as玩家控制器 (Utilities|Casting|CastToPlayerController (Pawn|GetController)))
  (Input|AddMappingContext (PlayerController|LocalPlayerSubsystems|GetEnhancedInputLocalPlayerSubsystem _as玩家控制器) "/Game/Default.Default" 0 "(bIgnoreAllPressedKeysUntilRelease=True,bForceImmediately=False,bNotifyUserSettings=False)")
  (Development|PrintString "Mapping Context Added")
  (bind _returnvalue (UserInterface|CreateWidget "/Game/CrossHair.CrossHair_C"))
  (UserInterface|Viewport|AddtoViewport _returnvalue 0))

(event Collision|EventActorBeginOverlap
  (params (OtherActor :type Actor%20Object%20Reference)))

(event EventEndPlay
  (params (EndPlayReason :type EEndPlayReason%20Enum :default "Destroyed")))

(event EventTick
  (params (DeltaSeconds :type Float%20%28single-precision%29))
  (bind _springarm (Variables|Default|GetSpringArm))
  (Variables|/Script/Engine.SpringArmComponent|SetSocketOffset _springarm (Math|Vector|MakeVector (.X (Math|Vector|BreakVector (Variables|/Script/Engine.SpringArmComponent|GetSocketOffset _springarm))) (Math|Interpolation|FInterpTo (.Y (Math|Vector|BreakVector (Variables|/Script/Engine.SpringArmComponent|GetSocketOffset _springarm))) (Variables|Default|GetShoulderY) (Utilities|Time|GetWorldDeltaSeconds) 8.0) (.Z (Math|Vector|BreakVector (Variables|/Script/Engine.SpringArmComponent|GetSocketOffset _springarm))))))

(fn ConstructionScript)
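; BP_MusicBox is an interactable music box that, once activated, repeatedly emits noise events for AI hearing.
; Interact sets IsPlaying and starts a looping timer on BoxMakeNoise, which calls MakeNoise and reports a tagged AI perception noise at the box's location, with nothing here stopping it.
; A trigger box shows a text label while BP_TestCharacterMerge overlaps, and Tick turns that label toward the character, looked up by class every frame.
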(event OnComponentBeginOverlap(Box1)
  (params (OverlappedComponent :type Primitive%20Component%20Object%20Reference) (OtherActor :type Actor%20Object%20Reference) (OtherComp :type Primitive%20Component%20Object%20Reference) (OtherBodyIndex :type Integer) (bFromSweep :type Boolean) (SweepResult :type Hit%20Result%20Structure%20%28by%20ref%29))
  (Utilities|Casting|CastToBP_TestCharacterMerge OtherActor)
  (Rendering|SetVisibility (Variables|Default|GetTextRender) true false))

(event OnComponentEndOverlap(Box1)
  (params (OverlappedComponent :type Primitive%20Component%20Object%20Reference) (OtherActor :type Actor%20Object%20Reference) (OtherComp :type Primitive%20Component%20Object%20Reference) (OtherBodyIndex :type Integer))
  (Utilities|Casting|CastToBP_TestCharacterMerge OtherActor)
  (Rendering|SetVisibility (Variables|Default|GetTextRender) false false))

(event EventBeginPlay)

(event Collision|EventActorBeginOverlap
  (params (OtherActor :type Actor%20Object%20Reference)))

(event EventTick
  (params (DeltaSeconds :type Float%20%28single-precision%29))
  (bind _textrender (Variables|Default|GetTextRender))
  (bind _returnvalue (Actor|GetActorOfClass "/Game/Characters/BP_TestCharacterMerge.BP_TestCharacterMerge_C"))
  (Transformation|SetWorldRotation _textrender (Math|Rotator|FindLookatRotation (Transformation|GetWorldLocation _textrender) (Transformation|GetWorldLocation (Variables|/Script/Engine.Actor|GetRootComponent _returnvalue))) false false))

(event EventInteract
  (params (Caller :type Actor%20Object%20Reference))
  (Development|PrintString "Interaction called")
  (if (not (Variables|Default|GetisPlaying))
    (Variables|Default|SetisPlaying true)
    (Development|PrintString "Music Box Activated!")
    (Utilities|Time|SetTimerbyFunctionName 0 "BoxMakeNoise" 0.5 true)))

(fn ConstructionScript)

(fn BoxMakeNoise
  (Class|Actor|MakeNoise 1.0 0 "0, 0, 0" 0.0 "None")
  (Class|AISenseHearing|ReportNoiseEvent (Transformation|GetActorLocation) 1.0 self 3e+03 "MusicBox")
  (Development|PrintString "Music Box Playing"))
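; Oxygen actor that acts as a save point for the state of the level's switches.
; On BeginPlay it gathers every Switch_BP into a list and builds a parallel list of saved flags, all initially false.
; Save copies each switch's IsRedirected into the matching index; nothing here restores those values.
; An Oxygen Wwise event node exists but is unconnected, so it never plays.
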(event EventBeginPlay
  (|CallParentFunction)
  ;[0.5573 0.5573 0.5573 0.5] Creates a list of switches and corresponding list of save states
  (bind _outactors (Actor|GetAllActorsOfClass "/Game/Interaction/Actors/Switch_BP.Switch_BP_C"))
  (for _array_element _outactors
    (Utilities|Array|Add (Variables|Default|GetSwitchList) _array_element)
    (Utilities|Array|Add (Variables|Default|GetSwitchSaveList) false)))

(event Collision|EventActorBeginOverlap
  (params (OtherActor :type Actor%20Object%20Reference))
  (|CallParentFunction OtherActor) ; This node is disabled and will not be called.\nDrag off pins to build functionality.
)

(event EventTick
  (params (DeltaSeconds :type Float%20%28single-precision%29))
  (|CallParentFunction DeltaSeconds) ; This node is disabled and will not be called.\nDrag off pins to build functionality.
)

(fn ConstructionScript
  (|CallParentFunction))

(fn Save
  ;[0.15 0.15 0.15 0.5] Stores current state of switches
  (for (_array_element _array_index) (Variables|Default|GetSwitchList)
    (Utilities|Array|SetArrayElem (Variables|Default|GetSwitchSaveList) _array_index (Variables|/Game/Interaction/Actors/Switch_BP.Switch_BP_C|GetisRedirected _array_element))))
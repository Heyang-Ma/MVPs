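; Lore pickup actor that flickers a rect light until read and can pass its text to the player character's text menu.
; Tick counts down in frames and toggles the light at random intervals, keeping it off once IsRead is set.
; TextTransfer finds the test character among the box's overlaps, re-fetches it by class, copies text, title and background onto it, then calls TextMenu.
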(event EventBeginPlay
  (|CallParentFunction) ; This node is disabled and will not be called.\nDrag off pins to build functionality.
)

(event Collision|EventActorBeginOverlap
  (params (OtherActor :type Actor%20Object%20Reference))
  (|CallParentFunction OtherActor) ; This node is disabled and will not be called.\nDrag off pins to build functionality.
)

(event EventTick
  (params (DeltaSeconds :type Float%20%28single-precision%29))
  (bind _rectlight (Variables|Default|GetRectLight))
  (|CallParentFunction DeltaSeconds)
  (Variables|Default|Settimer (- (Variables|Default|Gettimer) 1))
  (if (Variables|Default|GetisRead)
    (Rendering|SetVisibility (Variables|Default|GetRectLight) false false)
    (elif (<= (Variables|Default|Gettimer) 0)
      (if (Rendering|IsVisible (Variables|Default|GetRectLight))
        (Rendering|SetVisibility _rectlight false false)
        (else
          (Rendering|SetVisibility _rectlight true false)))
      (Variables|Default|Settimer (Math|Random|RandomIntegerinRange 5 20)))))

(fn ConstructionScript
  (|CallParentFunction))

(fn TextTransfer
  (for _array_element (Collision|GetOverlappingActors (Variables|Default|GetBox) 0 :!class /Script/Engine.PrimitiveComponent)
    (bind _asbp_test_character_merge (Utilities|Casting|CastToBP_TestCharacterMerge _array_element))
    (bind _returnvalue (Actor|GetActorOfClass (Utilities|GetClass _asbp_test_character_merge)))
    (Variables|/Game/Characters/BP_TestCharacterMerge.BP_TestCharacterMerge_C|SetCurrentText _returnvalue (Variables|Default|GetCurrentText))
    (Variables|/Game/Characters/BP_TestCharacterMerge.BP_TestCharacterMerge_C|SetCurrentTextTitle _returnvalue (Variables|Default|GetCurrentTextTitle))
    (Variables|/Game/Characters/BP_TestCharacterMerge.BP_TestCharacterMerge_C|SetLore_Background _returnvalue (Variables|Default|GetBackground))
    (Default|TextMenu _returnvalue)))
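; MusicBox_BP is an interactable music box actor that, once activated, repeatedly emits noise that AI can hear.
; InteractionEvent sets a one-shot IsPlaying flag and starts a looping half-second timer on BoxMakeNoise, with no stop logic.
; Each tick of that timer calls MakeNoise and reports a ranged, "MusicBox"-tagged hearing event at the actor's location.
; Feedback is debug prints only; no audio plays.
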(event EventBeginPlay
  (|CallParentFunction) ; This node is disabled and will not be called.\nDrag off pins to build functionality.
)

(event Collision|EventActorBeginOverlap
  (params (OtherActor :type Actor%20Object%20Reference))
  (|CallParentFunction OtherActor) ; This node is disabled and will not be called.\nDrag off pins to build functionality.
)

(event EventTick
  (params (DeltaSeconds :type Float%20%28single-precision%29))
  (|CallParentFunction DeltaSeconds) ; This node is disabled and will not be called.\nDrag off pins to build functionality.
)

(fn ConstructionScript
  (|CallParentFunction))

(fn InteractionEvent
  (Development|PrintString "Interaction called")
  (if (not (Variables|Default|GetisPlaying))
    (Variables|Default|SetisPlaying true)
    (Development|PrintString "Music Box Activated!")
    (Utilities|Time|SetTimerbyFunctionName 0 "BoxMakeNoise" 0.5 true)))

(fn BoxMakeNoise
  (Class|Actor|MakeNoise 1.0 0 "0, 0, 0" 0.0 "None")
  (Class|AISenseHearing|ReportNoiseEvent (Transformation|GetActorLocation) 1.0 self 3e+03 "MusicBox")
  (Development|PrintString "Music Box Playing"))
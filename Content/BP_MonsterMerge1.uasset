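; BP_MonsterMerge1 is a monster that damages the player by draining oxygen while they are inside its KillBox.
; Each Tick counts down a cooldown timer and polls KillBox for overlapping BP_TestCharacter actors, matching them against the one returned by GetActorOfClass.
; When the timer is below zero, a match loses a fixed amount of CurrentOxygen and the timer resets to TimerMax.
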(event EventTick
  (params (DeltaSeconds :type Float%20%28single-precision%29))
  ;[0.15 0.15 0.15 0.5] Update the damage cooldown timer
  (Variables|Default|Settimer (- (Variables|Default|Gettimer) DeltaSeconds))
  ;[0.15 0.15 0.15 0.5] Check overlapped object is player
  (for _array_element (Collision|GetOverlappingActors (Variables|Default|GetKillBox) "/Game/BP_TestCharacter.BP_TestCharacter_C" :!class /Script/Engine.PrimitiveComponent)
    (bind _returnvalue (Actor|GetActorOfClass "/Game/BP_TestCharacter.BP_TestCharacter_C"))
    (if (== _array_element _returnvalue)
      ;[0.15 0.15 0.15 0.5] Checking timer is finished
      (if (< (Variables|Default|Gettimer) 0.0)
        ;[0.15 0.15 0.15 0.5] Dealing Damage
        (bind _asbp_test_character (Utilities|Casting|CastToBP_TestCharacter _array_element))
        (Variables|/Game/BP_TestCharacter.BP_TestCharacter_C|SetCurrentOxygen _asbp_test_character (- (Variables|/Game/BP_TestCharacter.BP_TestCharacter_C|GetCurrentOxygen _asbp_test_character) 3e+01))
        ;[0.15 0.15 0.15 0.5] Reset Timer
        (Variables|Default|Settimer (Variables|Default|GettimerMax))))))

(fn ConstructionScript)
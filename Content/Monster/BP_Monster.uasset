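; Monster character that roams patrol routes and drains the player's oxygen to zero on sphere overlap.
; Tick sets CurrentTarget from one of four point arrays, picking a random route when one ends or the monster stops moving.
; Stun halts movement, shows electrocution VFX and sets AIC_Monster blackboard keys until a timed recovery.
; Tick also feeds idle state to the animation instance, and the suit mesh follows the body's pose.
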(event OnComponentBeginOverlap(Sphere)
  (params (OverlappedComponent :type Primitive%20Component%20Object%20Reference) (OtherActor :type Actor%20Object%20Reference) (OtherComp :type Primitive%20Component%20Object%20Reference) (OtherBodyIndex :type Integer) (bFromSweep :type Boolean) (SweepResult :type Hit%20Result%20Structure%20%28by%20ref%29))
  (bind _asbp_test_character_merge (Utilities|Casting|CastToBP_TestCharacterMerge OtherActor))
  (Variables|/Game/Characters/BP_TestCharacterMerge.BP_TestCharacterMerge_C|SetCurrentOxygen _asbp_test_character_merge 0.0))

(event Custom|Stun
  (Development|PrintString "Monster stunned!")
  (Components|Activation|SetActive (Variables|Default|GetNS_Electricution) true false)
  (bind _asaic_monster (Utilities|Casting|CastToAIC_Monster (Pawn|GetController)))
  (AI|Components|Blackboard|SetValueasBool (AI|GetBlackboard _asaic_monster) (Utilities|Name|MakeLiteralName "IsStunned") true)
  (Components|Movement|StopMovementImmediately (Variables|Character|GetCharacterMovement))
  (AI|Components|Blackboard|ClearValue (AI|GetBlackboard _asaic_monster) (Utilities|Name|MakeLiteralName "TargetActor"))
  (Utilities|Time|SetTimerbyEvent (delegate Custom|RecoverFromStun) 3.0))

(event Custom|RecoverFromStun
  (bind _asaic_monster (Utilities|Casting|CastToAIC_Monster (Pawn|GetController)))
  (AI|Components|Blackboard|SetValueasBool (AI|GetBlackboard _asaic_monster) (Utilities|Name|MakeLiteralName "IsStunned") false)
  (AI|Components|Blackboard|ClearValue (AI|GetBlackboard _asaic_monster) (Utilities|Name|MakeLiteralName "TargetActor"))
  (Development|PrintString "Monster recovered!")
  (Components|Activation|SetActive (Variables|Default|GetNS_Electricution) false false))

(event EventBeginPlay)

(event Collision|EventActorBeginOverlap
  (params (OtherActor :type Actor%20Object%20Reference)))

(event EventTick
  (params (DeltaSeconds :type Float%20%28single-precision%29))
  (bind _returnvalue (Transformation|GetVelocity))
  (bind _returnvalue_2 (Utilities|Operators|EqualEqual :A _returnvalue))
  (Utilities|FlowControl|Sequence
    (:then_0
      (Variables|Default|SetTimer (+ (Variables|Default|GetTimer) DeltaSeconds))
      (if (>= (Variables|Default|GetTimer) 3.0)
        (Variables|Default|SetTimer 0.0)
        (Variables|Default|SetLast%20Location (Transformation|GetActorLocation))))
    (:then_1
      (if (> (Variables|Default|GetTimer) 2.0)
        (if (Utilities|Operators|EqualEqual (Transformation|GetActorLocation) (Variables|Default|GetLast%20Location) 0.0)
          (Variables|Default|SetPatrol%20Pattern (Math|Random|RandomIntegerinRange 0 3))
          (Variables|Default|SetPatrol%20Point%20Index 0)
          (Development|PrintString "Monster reset"))))
    (:then_2
      (switch int (Variables|Default|GetPatrol%20Pattern)
        (:0
          (for (_array_element _array_index) (Variables|Default|GetPatrolPoints)
            (Utilities|FlowControl|Sequence
              (:then_0
                (if (== _array_index (Variables|Default|GetPatrol%20Point%20Index))
                  (Variables|Default|SetCurrentTarget _array_element)))
              (:then_1
                (if (> (Variables|Default|GetPatrol%20Point%20Index) (- (Utilities|Array|Length (Variables|Default|GetPatrolPoints)) 1))
                  (Variables|Default|SetPatrol%20Pattern (Math|Random|RandomIntegerinRange 0 3))
                  (Variables|Default|SetPatrol%20Point%20Index 0))))))
        (:1
          (for (_array_element_2 _array_index_2) (Variables|Default|GetPatrolPoints_0)
            (Utilities|FlowControl|Sequence
              (:then_0
                (if (== _array_index_2 (Variables|Default|GetPatrol%20Point%20Index))
                  (Variables|Default|SetCurrentTarget _array_element_2)))
              (:then_1
                (if (> (Variables|Default|GetPatrol%20Point%20Index) (- (Utilities|Array|Length (Variables|Default|GetPatrolPoints_0)) 1))
                  (Variables|Default|SetPatrol%20Pattern (Math|Random|RandomIntegerinRange 0 3))
                  (Variables|Default|SetPatrol%20Point%20Index 0))))))
        (:2
          (for (_array_element_3 _array_index_3) (Variables|Default|GetPatrolPoints_1)
            (Utilities|FlowControl|Sequence
              (:then_0
                (if (== _array_index_3 (Variables|Default|GetPatrol%20Point%20Index))
                  (Variables|Default|SetCurrentTarget _array_element_3)))
              (:then_1
                (if (> (Variables|Default|GetPatrol%20Point%20Index) (- (Utilities|Array|Length (Variables|Default|GetPatrolPoints_1)) 1))
                  (Variables|Default|SetPatrol%20Pattern (Math|Random|RandomIntegerinRange 0 3))
                  (Variables|Default|SetPatrol%20Point%20Index 0))))))
        (:3
          (for (_array_element_4 _array_index_4) (Variables|Default|GetPatrolPoints_2)
            (Utilities|FlowControl|Sequence
              (:then_0
                (if (== _array_index_4 (Variables|Default|GetPatrol%20Point%20Index))
                  (Variables|Default|SetCurrentTarget _array_element_4)))
              (:then_1
                (if (> (Variables|Default|GetPatrol%20Point%20Index) (- (Utilities|Array|Length (Variables|Default|GetPatrolPoints_2)) 1))
                  (Variables|Default|SetPatrol%20Pattern (Math|Random|RandomIntegerinRange 0 3))
                  (Variables|Default|SetPatrol%20Point%20Index 0))))))))
    (:then_3
      (Development|PrintString (Utilities|String|ToString(Boolean) _returnvalue_2))
      (bind _asstate_m_creature (Utilities|Casting|CastToStateM_Creature (Components|SkeletalMesh|GetAnimInstance (Variables|Character|GetMesh))))
      (if _returnvalue_2
        (Variables|/Game/Monster/Creature/StateM_Creature.StateM_Creature_C|SetisIdle _asstate_m_creature true)
        (else
          (Variables|/Game/Monster/Creature/StateM_Creature.StateM_Creature_C|SetisIdle _asstate_m_creature false))))))

(fn ConstructionScript
  (Components|SkinnedMesh|SetLeaderPoseComponent (Variables|Default|GetmonstermashSUIT) (Variables|Character|GetMesh) false false))
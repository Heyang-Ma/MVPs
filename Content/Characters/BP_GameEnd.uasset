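; BP_GameEnd is an end-of-game effects Blueprint that spawns fire and explosions, then returns to the main menu.
; GenerateFire starts a looping timer with no event shown bound and spawns several P_Fire emitters at random XY offsets around world origin.
; Explosion spawns P_Explosion emitters near origin, calling open level for Lvl_MainMenu inside the loop.
; The event graph is empty, so both functions rely on external callers.
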(event EventBeginPlay)

(event Collision|EventActorBeginOverlap
  (params (OtherActor :type Actor%20Object%20Reference)))

(event EventTick
  (params (DeltaSeconds :type Float%20%28single-precision%29)))

(fn ConstructionScript)

(fn GenerateFire
  (Utilities|Time|SetTimerbyEvent 0 1.0 true true)
  (for _index (range 0 6)
    (bind _returnvalue (Effects|SpawnEmitteratLocation "/Game/StarterContent/Particles/P_Fire.P_Fire" (Math|Vector|MakeVector (Math|Random|RandomFloatinRange -1e+02 1e+02) (Math|Random|RandomFloatinRange -1e+02 1e+02) 0.0)))
    (Variables|/Script/Engine.ParticleSystemComponent|SetSecondsBeforeInactive _returnvalue 1e+01)))

(fn Explosion
  (for _index (range 0 5)
    (Effects|SpawnEmitteratLocation "/Game/StarterContent/Particles/P_Explosion.P_Explosion" (Math|Vector|MakeVector (Math|Random|RandomFloatinRange -1e+01 1e+01) (Math|Random|RandomFloatinRange -1e+01 1e+01) (Math|Random|RandomFloatinRange -1e+01 1e+01)))
    (Game|OpenLevel(byObjectReference) "/Game/Craig_Work/Lvl_MainMenu.Lvl_MainMenu")))
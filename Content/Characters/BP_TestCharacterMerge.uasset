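; Player character with over-the-shoulder camera, crouch, stamina-limited sprint and a cooldown taser that stuns BP_Monster.
; Tick drives shoulder-swap interpolation, stamina, taser cooldown, their indicators, movement-scaled MakeNoise, and oxygen drain shown on the tank material.
; Empty oxygen triggers a delayed return to LastCheckpointLocation and restores saved switch states.
; Interact refills and saves at Oxygen_BP, transfers lore text, redirects switches, and messages the actor hit by a forward trace.
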(event Input|EnhancedActionEvents|EnhancedInputActionMove
  (params (ActionValue :type Vector%202D%20Structure) (ElapsedSeconds :type Float%20%28double-precision%29) (TriggeredSeconds :type Float%20%28double-precision%29) (InputAction :type Input%20Action%20Object%20Reference :default "/Game/Input/Move.Move"))
  (bind (_x _y) (Math|Vector2D|BreakVector2D ActionValue))
  (Pawn|Input|AddMovementInput (Transformation|GetActorForwardVector) _y false)
  (Pawn|Input|AddMovementInput (Transformation|GetActorRightVector) _x false))

(event Input|EnhancedActionEvents|EnhancedInputActionInteract
  (params (ActionValue :type Boolean) (ElapsedSeconds :type Float%20%28double-precision%29) (TriggeredSeconds :type Float%20%28double-precision%29) (InputAction :type Input%20Action%20Object%20Reference :default "/Game/Input/Interact.Interact"))
  (bind (_outlocation _outrotation) (Actor|GetActorEyesViewPoint))
  (Utilities|FlowControl|Sequence
    (:then_0
      ;[0.15 0.15 0.15 0.5] Interaction
      (Development|PrintString "Hello")
      ;;[0.75 0.75 0.75 0.5] Deciding whether you are interacting with an interactable
      (for _array_element (Collision|GetOverlappingActors (Variables|Collision|GetCapsuleComponent) "/Game/Interaction/Actors/InteractableParent_BP.InteractableParent_BP_C" :!class /Script/Engine.PrimitiveComponent)
        (bind _outactors (Actor|GetAllActorsOfClass "/Game/Interaction/Actors/InteractableParent_BP.InteractableParent_BP_C"))
        (for _array_element_2 _outactors
          (if (== _array_element_2 _array_element)
            (Utilities|FlowControl|Sequence
              (:then_0
                ;;[0.6875 0.6875 0.6875 0.5] Oxyegn Interaction
                (if (== "/Game/Interaction/Actors/Oxygen_BP.Oxygen_BP_C" (Utilities|GetClass _array_element_2))
                  (Variables|Default|SetCurrentOxygen (Variables|Default|GetMaxOxygen))
                  (bind _returnvalue (Actor|GetActorOfClass "/Game/Interaction/Actors/Oxygen_BP.Oxygen_BP_C"))
                  (Default|Save _returnvalue)))
              (:then_1
                ;;[0.7083 0.7083 0.7083 0.5] Lore Interaction
                (if (== "/Game/Interaction/Actors/Lore_BP.Lore_BP_C" (Utilities|GetClass _array_element_2))
                  (bind _outactors_2 (Actor|GetAllActorsOfClass "/Game/Interaction/Actors/Lore_BP.Lore_BP_C"))
                  (for _array_element_3 _outactors_2
                    (if (== _array_element_3 _array_element)
                      (Default|TextTransfer _array_element_3)))))
              (:then_2
                (if (== "/Game/Interaction/Actors/Switch_BP.Switch_BP_C" (Utilities|GetClass _array_element_2))
                  (bind _outactors_3 (Actor|GetAllActorsOfClass "/Game/Interaction/Actors/Switch_BP.Switch_BP_C"))
                  (for _array_element_4 _outactors_3
                    (if (== _array_element_4 _array_element)
                      (if (not (Variables|/Game/Interaction/Actors/Switch_BP.Switch_BP_C|GetisRedirected _array_element_4))
                        (Variables|/Game/Interaction/Actors/Switch_BP.Switch_BP_C|SetisRedirected _array_element_4 true)))))))))))
    (:then_1
      (Development|PrintString "E pressed")
      (bind _outhit (Collision|SphereTraceByChannel _outlocation (+ _outlocation (* (Math|Vector|GetForwardVector _outrotation) 3e+02)) 3e+01 "TraceTypeQuery1" false 0 "None"))
      (if true
        (Development|PrintString "Hit sth")
        (Class|Interactable|Interact(Message) (.HitActor (Collision|BreakHitResult _outhit)))
        (else
          (Development|PrintString "Didnt hit"))))))

(event Input|EnhancedActionEvents|EnhancedInputActionCrouch
  (params (ActionValue :type Boolean) (ElapsedSeconds :type Float%20%28double-precision%29) (TriggeredSeconds :type Float%20%28double-precision%29) (InputAction :type Input%20Action%20Object%20Reference :default "/Game/Input/Crouch.Crouch"))
  (:Started
    (Character|Crouch)
    (Variables|Default|SetIsCrouching true))
  (:Completed
    (Character|UnCrouch)
    (Variables|Default|SetIsCrouching false)))

(event Input|EnhancedActionEvents|EnhancedInputActionSwitch_Shoulder
  (params (ActionValue :type Boolean) (ElapsedSeconds :type Float%20%28double-precision%29) (TriggeredSeconds :type Float%20%28double-precision%29) (InputAction :type Input%20Action%20Object%20Reference :default "/Game/Input/Switch_Shoulder.Switch_Shoulder"))
  (:Started
    (Utilities|FlowControl|FlipFlop
      (:A
        (Variables|Default|SetShoulderY 6e+01))
      (:B
        (Variables|Default|SetShoulderY -6e+01)))))

(event Input|EnhancedActionEvents|EnhancedInputActionLookx
  (params (ActionValue :type Float%20%28double-precision%29) (ElapsedSeconds :type Float%20%28double-precision%29) (TriggeredSeconds :type Float%20%28double-precision%29) (InputAction :type Input%20Action%20Object%20Reference :default "/Game/Input/Lookx.Lookx"))
  (Pawn|Input|AddControllerYawInput ActionValue))

(event Input|EnhancedActionEvents|EnhancedInputActionLooky
  (params (ActionValue :type Float%20%28double-precision%29) (ElapsedSeconds :type Float%20%28double-precision%29) (TriggeredSeconds :type Float%20%28double-precision%29) (InputAction :type Input%20Action%20Object%20Reference :default "/Game/Input/Looky.Looky"))
  (Pawn|Input|AddControllerPitchInput ActionValue))

(event Input|EnhancedActionEvents|EnhancedInputActionSprint
  (params (ActionValue :type Boolean) (ElapsedSeconds :type Float%20%28double-precision%29) (TriggeredSeconds :type Float%20%28double-precision%29) (InputAction :type Input%20Action%20Object%20Reference :default "/Game/Input/Sprint.Sprint"))
  (bind _charactermovement (Variables|Character|GetCharacterMovement))
  (:Started
    (Variables|/Script/Engine.CharacterMovementComponent|SetMaxWalkSpeed _charactermovement 8.5e+02)
    (Variables|Default|SetIsSprint true)
    (Variables|Default|SetStaminaConsume 14.0)
    (Variables|Default|SetSprintingEndTime 0.0))
  (:Completed
    (Variables|/Script/Engine.CharacterMovementComponent|SetMaxWalkSpeed _charactermovement 5e+02)
    (Variables|Default|SetIsSprint false)
    (Variables|Default|SetStaminaConsume 0.0)
    (Variables|Default|SetStaminaRecovery 15.0)))

(event Input|EnhancedActionEvents|EnhancedInputActionTaser
  (params (ActionValue :type Boolean) (ElapsedSeconds :type Float%20%28double-precision%29) (TriggeredSeconds :type Float%20%28double-precision%29) (InputAction :type Input%20Action%20Object%20Reference :default "/Game/Input/Taser.Taser"))
  (bind _returnvalue (Game|GetPlayerCameraManager 0))
  (bind _taserrange (Variables|Default|GetTaserRange))
  (bind _arrow1 (Variables|Default|GetArrow1))
  (bind _ns_tasershot (Variables|Default|GetNS_TaserShot))
  (bind _returnvalue_2 (Camera|GetCameraLocation _returnvalue))
  (bind _returnvalue_3 (Camera|GetCameraRotation _returnvalue))
  (bind _returnvalue_4 (Transformation|GetWorldLocation _arrow1))
  (bind _returnvalue_5 (Math|Vector|GetForwardVector _returnvalue_3))
  (bind _returnvalue_6 (* _returnvalue_5 _taserrange))
  (bind _returnvalue_7 (+ _returnvalue_2 _returnvalue_6))
  (:Started
    (if (Variables|Default|GetCanFire)
      (bind (_outhit _returnvalue_8) (Collision|SphereTraceByChannel _returnvalue_4 _returnvalue_7 15.0 "TraceTypeQuery2" false (Utilities|Array|MakeArray self) "None"))
      ;[0.8177 0.8177 0.8177 0.5] FX For Taser Shot
      (Niagara|SetNiagaraVariable(Vector3) _ns_tasershot "Location Start" _returnvalue_4)
      (Niagara|SetNiagaraVariable(Vector3) _ns_tasershot "Location End" _returnvalue_7)
      (Variables|Default|SetTaserShotVFXTimer 0.0)
      (Components|Activation|SetActive _ns_tasershot true false)
      (if _returnvalue_8
        (bind _asbp_monster (Utilities|Casting|CastToBP_Monster (.HitActor (Collision|BreakHitResult _outhit)))
          (:then
            (Default|Stun _asbp_monster)
            (Development|PrintString "Monster Hit")
            (Variables|Default|SetCanFire false)
            (Variables|Default|SetCurrentTaserCooldown (Variables|Default|GetTaserCooldown)))
          (:CastFailed
            (Development|PrintString "Hit other things")))
        (else
          (Development|PrintString "Miss: Out of range")
          (Variables|Default|SetCanFire false)
          (Variables|Default|SetCurrentTaserCooldown (Variables|Default|GetTaserCooldown)))))))

(event EventBeginPlay
  (Variables|Default|SetCurrentStamina (Variables|Default|GetMaxStamina))
  (bind _asplayer_controller (Utilities|Casting|CastToPlayerController (Pawn|GetController)))
  (Input|AddMappingContext (PlayerController|LocalPlayerSubsystems|GetEnhancedInputLocalPlayerSubsystem _asplayer_controller) "/Game/Input/Default.Default" 0 "(bIgnoreAllPressedKeysUntilRelease=True,bForceImmediately=False,bNotifyUserSettings=False)")
  (Development|PrintString "Mapping Context Added")
  (bind _returnvalue (UserInterface|CreateWidget "/Game/UI/CrossHair.CrossHair_C"))
  (UserInterface|Viewport|AddtoViewport _returnvalue 0)
  (bind _returnvalue_2 (Rendering|Material|CreateDynamicMaterialInstance (Variables|Default|GetOxygenTank) 0 0 "None" :!class /Script/Engine.PrimitiveComponent))
  (Variables|Default|SetOxygenMaterial _returnvalue_2)
  (Variables|Default|SetLastCheckpointLocation (Transformation|GetActorLocation))
  (bind _astaser_charge (Utilities|Casting|CastToTaserCharge (UserInterface|GetWidget (Variables|Default|GetTaserChargeWidget))))
  (Variables|Default|SetTaserChargeWidgetRef _astaser_charge))

(event Collision|EventActorBeginOverlap
  (params (OtherActor :type Actor%20Object%20Reference)))

(event EventEndPlay
  (params (EndPlayReason :type EEndPlayReason%20Enum :default "Destroyed")))

(event EventTick
  (params (DeltaSeconds :type Float%20%28single-precision%29))
  (bind _springarm (Variables|Default|GetSpringArm))
  (bind _taserchargewidgetref (Variables|Default|GetTaserChargeWidgetRef))
  (bind _staminawheel (Variables|Default|GetStaminaWheel))
  (bind _oxygenmaterial (Variables|Default|GetOxygenMaterial))
  (Utilities|FlowControl|Sequence
    (:then_0
      (Variables|/Script/Engine.SpringArmComponent|SetSocketOffset _springarm (Math|Vector|MakeVector (.X (Math|Vector|BreakVector (Variables|/Script/Engine.SpringArmComponent|GetSocketOffset _springarm))) (Math|Interpolation|FInterpTo (.Y (Math|Vector|BreakVector (Variables|/Script/Engine.SpringArmComponent|GetSocketOffset _springarm))) (Variables|Default|GetShoulderY) (Utilities|Time|GetWorldDeltaSeconds) 8.0) (.Z (Math|Vector|BreakVector (Variables|/Script/Engine.SpringArmComponent|GetSocketOffset _springarm))))))
    (:then_1
      (Variables|Default|SetCurrentOxygen (Math|Float|Clamp(Float) (- (Variables|Default|GetCurrentOxygen) (* (Variables|Default|GetOxygenDrainRate) DeltaSeconds)) 0.0 85.0))
      (Rendering|Material|SetScalarParameterValue _oxygenmaterial "FillAmount" (/ (Variables|Default|GetCurrentOxygen) (Variables|Default|GetMaxOxygen)) :!class /Script/Engine.MaterialInstanceDynamic)
      (Rendering|Material|SetScalarParameterValue _oxygenmaterial "ColourBlend" (- 1.0 (/ (Variables|Default|GetCurrentOxygen) (Variables|Default|GetMaxOxygen))) :!class /Script/Engine.MaterialInstanceDynamic)
      (if (and (<= (Variables|Default|GetCurrentOxygen) 0.0) (not (Variables|Default|GetIsDead)))
        (Variables|Default|SetIsDead true)
        (Utilities|FlowControl|Delay 2.0)
        (Transformation|SetActorLocation (Variables|Default|GetLastCheckpointLocation) false false)
        ;[0.474 0.474 0.474 0.5] Sets the switches to match their state when last saved
        (bind _returnvalue (Actor|GetActorOfClass "/Game/Interaction/Actors/Oxygen_BP.Oxygen_BP_C"))
        (for (_array_element _array_index) (Variables|/Game/Interaction/Actors/Oxygen_BP.Oxygen_BP_C|GetSwitchList _returnvalue)
          (Variables|/Game/Interaction/Actors/Switch_BP.Switch_BP_C|SetisRedirected _array_element (Utilities|Array|Get(acopy) (Variables|/Game/Interaction/Actors/Oxygen_BP.Oxygen_BP_C|GetSwitchSaveList _returnvalue) _array_index))
          (Variables|Default|SetCurrentOxygen (Variables|Default|GetMaxOxygen))
          (Variables|Default|SetIsDead false))))
    (:then_2
      (if (Variables|Default|GetIsSprint)
        (Variables|Default|SetCurrentStamina (Math|Float|Clamp(Float) (- (Variables|Default|GetCurrentStamina) (* (Variables|Default|GetStaminaConsume) (Utilities|Time|GetWorldDeltaSeconds))) 0.0 (Variables|Default|GetMaxStamina)))
        (else
          (Variables|Default|SetSprintingEndTime (+ (Variables|Default|GetSprintingEndTime) (Utilities|Time|GetWorldDeltaSeconds)))
          (if (>= (Variables|Default|GetSprintingEndTime) 4.0)
            (Variables|Default|SetCurrentStamina (Math|Float|Clamp(Float) (+ (Variables|Default|GetCurrentStamina) (* (Variables|Default|GetStaminaRecovery) (Utilities|Time|GetWorldDeltaSeconds))) 0.0 (Variables|Default|GetMaxStamina)))))))
    (:then_3
      (if (== (Variables|Default|GetCurrentStamina) 0.0)
        (Variables|/Script/Engine.CharacterMovementComponent|SetMaxWalkSpeed (Variables|Character|GetCharacterMovement) 5e+02)))
    (:then_4
      ;[0.15 0.15 0.15 0.5] Sound Creation
      (if (> (Math|Vector|VectorLength (Transformation|GetVelocity)) 1e+01)
        (if (Variables|Default|GetIsCrouching)
          (Class|Actor|MakeNoise 0.25 self "0, 0, 0" 0.0 "None")
          (elif (Variables|Default|GetIsSprint)
            (Class|Actor|MakeNoise 1.0 self "0, 0, 0" 0.0 "None")
            (else
              (Class|Actor|MakeNoise 0.5 self "0, 0, 0" 0.0 "None"))))))
    (:then_5
      ;[0.15 0.15 0.15 0.5] Stamina Wheel
      (Transformation|SetWorldLocation (Variables|Default|GetStaminaWheel) (Transformation|GetWorldLocation (Variables|Default|GetStamina%20Wheel%20Position)) false false)
      (bind _returnvalue_2 (Rendering|Material|CreateDynamicMaterialInstance (Variables|Default|GetStaminaWheel) 0 "/Game/UI/Stamina_Wheel/StaminaWheel_Mat.StaminaWheel_Mat" "None" :!class /Script/Engine.PrimitiveComponent))
      (Rendering|Material|SetScalarParameterValue _returnvalue_2 "Percentage" (Variables|Default|GetCurrentStamina) :!class /Script/Engine.MaterialInstanceDynamic)
      (if (== (Variables|Default|GetCurrentStamina) (Variables|Default|GetMaxStamina))
        (Rendering|SetVisibility _staminawheel false false)
        (else
          (Rendering|SetVisibility _staminawheel true false))))
    (:then_6
      (if (not (Variables|Default|GetCanFire))
        (Components|Activation|SetActive (Variables|Default|GetNS_TaserCharge) false false)
        (Variables|Default|SetCurrentTaserCooldown (- (Variables|Default|GetCurrentTaserCooldown) (Utilities|Time|GetWorldDeltaSeconds)))
        (if (Utilities|IsValid _taserchargewidgetref)
          (Default|UpdateCharge _taserchargewidgetref (- 1.0 (/ (Variables|Default|GetCurrentTaserCooldown) (Variables|Default|GetTaserCooldown))))
          (if (<= (Variables|Default|GetCurrentTaserCooldown) 0.0)
            (Variables|Default|SetCanFire true)))
        (else
          (Components|Activation|SetActive (Variables|Default|GetTaserChargeWidget) true false))))
    (:then_7
      ;[0.5417 0.5417 0.5417 0.5] Handling FX for Taser shot
      (bind _output_get (Variables|Default|SetTaserShotVFXTimer (+ (Variables|Default|GetTaserShotVFXTimer) DeltaSeconds)))
      (if (> _output_get 0.2)
        (Components|Activation|SetActive (Variables|Default|GetNS_TaserShot) false false)))))

(fn ConstructionScript)

(fn TextMenu
  (bind _foundwidgets (Widget|GetAllWidgetsOfClass "/Game/UI/Text.Text_C" true))
  (if (Utilities|IsValid (Utilities|Array|Get(acopy) _foundwidgets))
    ;[0.599 0.599 0.599 0.5] Alternating Text Menu State
    (if (Variables|Default|GetIsTextActive)
      (Widget|RemovefromParent (Utilities|Array|Get(acopy) _foundwidgets))
      (Variables|Default|SetIsTextActive false)
      (else
        (UserInterface|Viewport|AddtoViewport (Utilities|Array|Get(acopy) _foundwidgets) 0)
        (Variables|Default|SetIsTextActive true)))
    (else
      ;[0.5104 0.5104 0.5104 0.5] Creating widget
      (bind _returnvalue (UserInterface|CreateWidget "/Game/UI/Text.Text_C" (Game|GetPlayerController 0)))
      (UserInterface|Viewport|AddtoViewport _returnvalue 0)
      (Variables|Default|SetIsTextActive true))))
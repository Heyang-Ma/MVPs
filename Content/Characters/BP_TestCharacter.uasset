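; Third-person player character with movement, shoulder-swap camera, crouch, sprint stamina and draining oxygen.
; Tick interpolates the spring arm offset, updates stamina, drives the oxygen tank's dynamic material and teleports to the BeginPlay location after oxygen runs out.
; It also emits movement noise scaled by stance and feeds taser cooldown to a charge widget.
; The taser's line-trace stun of BP_Monster is disconnected and never runs.
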(event Input|EnhancedActionEvents|EnhancedInputActionMove
  (params (ActionValue :type Vector%202D%20Structure) (ElapsedSeconds :type Float%20%28double-precision%29) (TriggeredSeconds :type Float%20%28double-precision%29) (InputAction :type Input%20Action%20Object%20Reference :default "/Game/Input/Move.Move"))
  (bind (_x _y) (Math|Vector2D|BreakVector2D ActionValue))
  (Pawn|Input|AddMovementInput (Transformation|GetActorForwardVector) _y false)
  (Pawn|Input|AddMovementInput (Transformation|GetActorRightVector) _x false))

(event Input|EnhancedActionEvents|EnhancedInputActionSprint
  (params (ActionValue :type Boolean) (ElapsedSeconds :type Float%20%28double-precision%29) (TriggeredSeconds :type Float%20%28double-precision%29) (InputAction :type Input%20Action%20Object%20Reference :default "/Game/Input/Sprint.Sprint"))
  (bind _charactermovement (Variables|Character|GetCharacterMovement))
  (:Started
    (Variables|/Script/Engine.CharacterMovementComponent|SetMaxWalkSpeed _charactermovement 8.5e+02)
    (Variables|Default|SetIsSprint true)
    (Variables|Default|SetStaminaConsume 14.0)
    (Variables|Default|SetSprintingEndTime 0.0))
  (:Completed
    (Variables|/Script/Engine.CharacterMovementComponent|SetMaxWalkSpeed _charactermovement 3e+02)
    (Variables|Default|SetIsSprint false)
    (Variables|Default|SetStaminaConsume 0.0)
    (Variables|Default|SetStaminaRecovery 7.0)))

(event Input|EnhancedActionEvents|EnhancedInputActionCrouch
  (params (ActionValue :type Boolean) (ElapsedSeconds :type Float%20%28double-precision%29) (TriggeredSeconds :type Float%20%28double-precision%29) (InputAction :type Input%20Action%20Object%20Reference :default "/Game/Input/Crouch.Crouch"))
  (:Started
    (Character|Crouch)
    (Variables|Default|SetIsCrouching true))
  (:Completed
    (Character|UnCrouch)
    (Variables|Default|SetIsCrouching false)))

(event Input|EnhancedActionEvents|EnhancedInputActionSwitch_Shoulder
  (params (ActionValue :type Boolean) (ElapsedSeconds :type Float%20%28double-precision%29) (TriggeredSeconds :type Float%20%28double-precision%29) (InputAction :type Input%20Action%20Object%20Reference :default "/Game/Input/Switch_Shoulder.Switch_Shoulder"))
  (:Started
    (Utilities|FlowControl|FlipFlop
      (:A
        (Variables|Default|SetShoulderY 6e+01))
      (:B
        (Variables|Default|SetShoulderY -6e+01)))))

(event Input|EnhancedActionEvents|EnhancedInputActionLookx
  (params (ActionValue :type Float%20%28double-precision%29) (ElapsedSeconds :type Float%20%28double-precision%29) (TriggeredSeconds :type Float%20%28double-precision%29) (InputAction :type Input%20Action%20Object%20Reference :default "/Game/Input/Lookx.Lookx"))
  (Pawn|Input|AddControllerYawInput ActionValue))

(event Input|EnhancedActionEvents|EnhancedInputActionLooky
  (params (ActionValue :type Float%20%28double-precision%29) (ElapsedSeconds :type Float%20%28double-precision%29) (TriggeredSeconds :type Float%20%28double-precision%29) (InputAction :type Input%20Action%20Object%20Reference :default "/Game/Input/Looky.Looky"))
  (Pawn|Input|AddControllerPitchInput ActionValue))

(event EventBeginPlay
  (Variables|Default|SetCurrentStamina (Variables|Default|GetMaxStamina))
  (bind _asplayer_controller (Utilities|Casting|CastToPlayerController (Pawn|GetController)))
  (Input|AddMappingContext (PlayerController|LocalPlayerSubsystems|GetEnhancedInputLocalPlayerSubsystem _asplayer_controller) "/Game/Input/Default.Default" 0 "(bIgnoreAllPressedKeysUntilRelease=True,bForceImmediately=False,bNotifyUserSettings=False)")
  (bind _returnvalue (UserInterface|CreateWidget "/Game/UI/StaminaBar.StaminaBar_C"))
  (UserInterface|Viewport|AddtoViewport _returnvalue 0)
  (bind _returnvalue_2 (UserInterface|CreateWidget "/Game/UI/CrossHair.CrossHair_C"))
  (UserInterface|Viewport|AddtoViewport _returnvalue_2 0)
  (bind _returnvalue_3 (Rendering|Material|CreateDynamicMaterialInstance (Variables|Default|GetOxygenTank) 0 0 "None" :!class /Script/Engine.PrimitiveComponent))
  (Variables|Default|SetOxygenMaterial _returnvalue_3)
  (Variables|Default|SetLastCheckpointLocation (Transformation|GetActorLocation))
  (bind _astaser_charge (Utilities|Casting|CastToTaserCharge (UserInterface|GetWidget (Variables|Default|GetTaserChargeWidget))))
  (Variables|Default|SetTaserChargeWidgetRef _astaser_charge))

(event Collision|EventActorBeginOverlap
  (params (OtherActor :type Actor%20Object%20Reference)))

(event EventEndPlay
  (params (EndPlayReason :type EEndPlayReason%20Enum :default "Destroyed")))

(event EventTick
  (params (DeltaSeconds :type Float%20%28single-precision%29))
  (bind _springarm (Variables|Default|GetSpringArm))
  (bind _taserchargewidgetref (Variables|Default|GetTaserChargeWidgetRef))
  (bind _oxygenmaterial (Variables|Default|GetOxygenMaterial))
  (Utilities|FlowControl|Sequence
    (:then_0
      (Variables|/Script/Engine.SpringArmComponent|SetSocketOffset _springarm (Math|Vector|MakeVector (.X (Math|Vector|BreakVector (Variables|/Script/Engine.SpringArmComponent|GetSocketOffset _springarm))) (Math|Interpolation|FInterpTo (.Y (Math|Vector|BreakVector (Variables|/Script/Engine.SpringArmComponent|GetSocketOffset _springarm))) (Variables|Default|GetShoulderY) (Utilities|Time|GetWorldDeltaSeconds) 8.0) (.Z (Math|Vector|BreakVector (Variables|/Script/Engine.SpringArmComponent|GetSocketOffset _springarm))))))
    (:then_1
      (Variables|Default|SetCurrentOxygen (Math|Float|Clamp(Float) (- (Variables|Default|GetCurrentOxygen) (* (Variables|Default|GetOxygenDrainRate) DeltaSeconds)) 0.0 1e+02))
      (Rendering|Material|SetScalarParameterValue _oxygenmaterial "FillAmount" (/ (Variables|Default|GetCurrentOxygen) (Variables|Default|GetMaxOxygen)) :!class /Script/Engine.MaterialInstanceDynamic)
      (Rendering|Material|SetScalarParameterValue _oxygenmaterial "ColourBlend" (- 1.0 (/ (Variables|Default|GetCurrentOxygen) (Variables|Default|GetMaxOxygen))) :!class /Script/Engine.MaterialInstanceDynamic)
      (if (and (<= (Variables|Default|GetCurrentOxygen) 0.0) (not (Variables|Default|GetIsDead)))
        (Variables|Default|SetIsDead true)
        (Utilities|FlowControl|Delay 2.0)
        (Transformation|SetActorLocation (Variables|Default|GetLastCheckpointLocation) false false)
        (Variables|Default|SetCurrentOxygen (Variables|Default|GetMaxOxygen))
        (Variables|Default|SetIsDead false)))
    (:then_2
      (if (Variables|Default|GetIsSprint)
        (bind _output_get (Variables|Default|SetCurrentStamina (Math|Float|Clamp(Float) (- (Variables|Default|GetCurrentStamina) (* (Variables|Default|GetStaminaConsume) (Utilities|Time|GetWorldDeltaSeconds))) 0.0 (Variables|Default|GetMaxStamina))))
        (Development|PrintString (Utilities|String|ToString(Float) _output_get) true true "(R=1.000000,G=0.687881,B=0.050316,A=1.000000)" 0.0)
        (else
          (Variables|Default|SetSprintingEndTime (+ (Variables|Default|GetSprintingEndTime) (Utilities|Time|GetWorldDeltaSeconds)))
          (if (>= (Variables|Default|GetSprintingEndTime) 3.0)
            (bind _output_get_2 (Variables|Default|SetCurrentStamina (Math|Float|Clamp(Float) (+ (Variables|Default|GetCurrentStamina) (* (Variables|Default|GetStaminaRecovery) (Utilities|Time|GetWorldDeltaSeconds))) 0.0 (Variables|Default|GetMaxStamina))))
            (Development|PrintString (Utilities|String|ToString(Float) _output_get_2) true true "(R=1.000000,G=0.099532,B=0.127229,A=1.000000)" 0.0)))))
    (:then_3
      (if (== (Variables|Default|GetCurrentStamina) 0.0)
        (Variables|/Script/Engine.CharacterMovementComponent|SetMaxWalkSpeed (Variables|Character|GetCharacterMovement) 3e+02)))
    (:then_4
      (if (> (Math|Vector|VectorLength (Transformation|GetVelocity)) 1e+01)
        (if (Variables|Default|GetIsCrouching)
          (Class|Actor|MakeNoise 0.25 self "0, 0, 0" 0.0 "None")
          (Development|PrintString "crouch: 5m noise")
          (elif (Variables|Default|GetIsSprint)
            (Class|Actor|MakeNoise 1.0 self "0, 0, 0" 0.0 "None")
            (Development|PrintString "run: 20m noise")
            (else
              (Class|Actor|MakeNoise 0.5 self "0, 0, 0" 0.0 "None")
              (Development|PrintString "walk: 10m noise"))))))
    (:then_5
      (if (not (Variables|Default|GetCanFire))
        (Variables|Default|SetCurrentCooldown (- (Variables|Default|GetCurrentCooldown) (Utilities|Time|GetWorldDeltaSeconds)))
        (if (Utilities|IsValid _taserchargewidgetref)
          (Development|PrintString "Updating charge")
          (Default|UpdateCharge _taserchargewidgetref (- 1.0 (/ (Variables|Default|GetCurrentCooldown) (Variables|Default|GetTaserCooldown))))
          (if (<= (Variables|Default|GetCurrentCooldown) 0.0)
            (Variables|Default|SetCanFire true)
            (Development|PrintString "Ready")))))))

(fn ConstructionScript)
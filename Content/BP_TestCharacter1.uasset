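; Player character with Enhanced Input movement, crouch, sprint, shoulder-swap camera and a draining oxygen supply shown on the tank's dynamic material.
; Tick eases the camera offset, updates stamina with delayed recovery, and handles oxygen depletion by returning to the BeginPlay location and restoring saved switch states.
; Interact checks overlapping InteractableParent_BP actors: oxygen refills and saves, lore transfers text, switches toggle redirection.
; TextMenu toggles a text widget.
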(event Input|EnhancedActionEvents|EnhancedInputActionMove
  (params (ActionValue :type Vector%202D%20Structure) (ElapsedSeconds :type Float%20%28double-precision%29) (TriggeredSeconds :type Float%20%28double-precision%29) (InputAction :type Input%20Action%20Object%20Reference :default "/Game/Move.Move"))
  (bind (_x _y) (Math|Vector2D|BreakVector2D ActionValue))
  (Pawn|Input|AddMovementInput (Transformation|GetActorForwardVector) _y false)
  (Pawn|Input|AddMovementInput (Transformation|GetActorRightVector) _x false))

(event Input|EnhancedActionEvents|EnhancedInputActionInteract
  (params (ActionValue :type Boolean) (ElapsedSeconds :type Float%20%28double-precision%29) (TriggeredSeconds :type Float%20%28double-precision%29) (InputAction :type Input%20Action%20Object%20Reference :default "/Game/Interact.Interact"))
  ;[0.15 0.15 0.15 0.5] Interaction
  ;;[0.75 0.75 0.75 0.5] Deciding whether you are interacting with an interactable
  (Development|PrintString "Hello")
  (for _array_element (Collision|GetOverlappingActors (Variables|Collision|GetCapsuleComponent) "/Game/Interaction/Actors/InteractableParent_BP.InteractableParent_BP_C" :!class /Script/Engine.PrimitiveComponent)
    (bind _outactors (Actor|GetAllActorsOfClass "/Game/Interaction/Actors/InteractableParent_BP.InteractableParent_BP_C"))
    (for _array_element_2 _outactors
      (if (== _array_element_2 _array_element)
        ;;[1 1 1 0.5] Interaction Effect
        (Development|PrintString (Variables|/Game/Interaction/Actors/InteractableParent_BP.InteractableParent_BP_C|GetTestText _array_element_2))
        (Utilities|FlowControl|Sequence
          (:then_0
            ;;[0.6875 0.6875 0.6875 0.5] Oxyegn Interaction
            (if (== "/Game/Interaction/Actors/Oxygen_BP.Oxygen_BP_C" (Utilities|GetClass _array_element_2))
              (Variables|Default|SetCurrentOxygen (Variables|Default|GetMaxOxygen))
              (bind _returnvalue (Actor|GetActorOfClass "/Game/Interaction/Actors/Oxygen_BP.Oxygen_BP_C"))
              (Default|Save _returnvalue)))
          (:then_1
            ;;[0.7083 0.7083 0.7083 0.5] Lore Interaction
            (if (== "/Game/Interaction/Actors/Lore_BP.Lore_BP_C" (Utilities|GetClass _array_element_2))
              (bind _outactors_2 (Actor|GetAllActorsOfClass "/Game/Interaction/Actors/Lore_BP.Lore_BP_C"))
              (for _array_element_3 _outactors_2
                (if (== _array_element_3 _array_element)
                  (Default|TextTransfer _array_element_3)))))
          (:then_2
            (if (== "/Game/Interaction/Actors/Switch_BP.Switch_BP_C" (Utilities|GetClass _array_element_2))
              (bind _outactors_3 (Actor|GetAllActorsOfClass "/Game/Interaction/Actors/Switch_BP.Switch_BP_C"))
              (for _array_element_4 _outactors_3
                (if (== _array_element_4 _array_element)
                  (if (Variables|/Game/Interaction/Actors/Switch_BP.Switch_BP_C|GetisRedirected _array_element_4)
                    (bind _output_get (Variables|/Game/Interaction/Actors/Switch_BP.Switch_BP_C|SetisRedirected _array_element_4 false))
                    (Development|PrintString (Utilities|String|ToString(Boolean) _output_get))
                    (else
                      (bind _output_get_2 (Variables|/Game/Interaction/Actors/Switch_BP.Switch_BP_C|SetisRedirected _array_element_4 true))
                      (Development|PrintString (Utilities|String|ToString(Boolean) _output_get_2)))))))))))))

(event Input|EnhancedActionEvents|EnhancedInputActionCrouch
  (params (ActionValue :type Boolean) (ElapsedSeconds :type Float%20%28double-precision%29) (TriggeredSeconds :type Float%20%28double-precision%29) (InputAction :type Input%20Action%20Object%20Reference :default "/Game/Crouch.Crouch"))
  (:Started
    (Development|PrintString "Crouch Pressed")
    (Character|Crouch))
  (:Completed
    (Character|UnCrouch)))

(event Input|EnhancedActionEvents|EnhancedInputActionSwitch_Shoulder
  (params (ActionValue :type Boolean) (ElapsedSeconds :type Float%20%28double-precision%29) (TriggeredSeconds :type Float%20%28double-precision%29) (InputAction :type Input%20Action%20Object%20Reference :default "/Game/Switch_Shoulder.Switch_Shoulder"))
  (:Started
    (Utilities|FlowControl|FlipFlop
      (:A
        (Variables|Default|SetShoulderY 6e+01))
      (:B
        (Variables|Default|SetShoulderY -6e+01)))))

(event Input|EnhancedActionEvents|EnhancedInputActionLookx
  (params (ActionValue :type Float%20%28double-precision%29) (ElapsedSeconds :type Float%20%28double-precision%29) (TriggeredSeconds :type Float%20%28double-precision%29) (InputAction :type Input%20Action%20Object%20Reference :default "/Game/Lookx.Lookx"))
  (Pawn|Input|AddControllerYawInput ActionValue))

(event Input|EnhancedActionEvents|EnhancedInputActionLooky
  (params (ActionValue :type Float%20%28double-precision%29) (ElapsedSeconds :type Float%20%28double-precision%29) (TriggeredSeconds :type Float%20%28double-precision%29) (InputAction :type Input%20Action%20Object%20Reference :default "/Game/Looky.Looky"))
  (Pawn|Input|AddControllerPitchInput ActionValue))

(event Input|EnhancedActionEvents|EnhancedInputActionSprint
  (params (ActionValue :type Boolean) (ElapsedSeconds :type Float%20%28double-precision%29) (TriggeredSeconds :type Float%20%28double-precision%29) (InputAction :type Input%20Action%20Object%20Reference :default "/Game/Sprint.Sprint"))
  (bind _charactermovement (Variables|Character|GetCharacterMovement))
  (:Started
    (Variables|/Script/Engine.CharacterMovementComponent|SetMaxWalkSpeed _charactermovement 8.5e+02)
    (Variables|Default|SetIsSprint true)
    (Variables|Default|SetStaminaConsume 14.0)
    (Variables|Default|SetSprintingEndTime 0.0))
  (:Completed
    (Variables|/Script/Engine.CharacterMovementComponent|SetMaxWalkSpeed _charactermovement 5e+02)
    (Variables|Default|SetIsSprint false)
    (Variables|Default|SetStaminaConsume 0.0)
    (Variables|Default|SetStaminaRecovery 15.0)))

(event EventBeginPlay
  (Variables|Default|SetCurrentStamina (Variables|Default|GetMaxStamina))
  (bind _asplayer_controller (Utilities|Casting|CastToPlayerController (Pawn|GetController)))
  (Input|AddMappingContext (PlayerController|LocalPlayerSubsystems|GetEnhancedInputLocalPlayerSubsystem _asplayer_controller) "/Game/Default.Default" 0 "(bIgnoreAllPressedKeysUntilRelease=True,bForceImmediately=False,bNotifyUserSettings=False)")
  (Development|PrintString "Mapping Context Added")
  (bind _returnvalue (UserInterface|CreateWidget "/Game/StaminaBar.StaminaBar_C"))
  (UserInterface|Viewport|AddtoViewport _returnvalue 0)
  (bind _returnvalue_2 (UserInterface|CreateWidget "/Game/CrossHair.CrossHair_C"))
  (UserInterface|Viewport|AddtoViewport _returnvalue_2 0)
  (bind _returnvalue_3 (Rendering|Material|CreateDynamicMaterialInstance (Variables|Default|GetOxygenTank) 0 0 "None" :!class /Script/Engine.PrimitiveComponent))
  (Variables|Default|SetOxygenMaterial _returnvalue_3)
  (Variables|Default|SetLastCheckpointLocation (Transformation|GetActorLocation)))

(event Collision|EventActorBeginOverlap
  (params (OtherActor :type Actor%20Object%20Reference)))

(event EventEndPlay
  (params (EndPlayReason :type EEndPlayReason%20Enum :default "Destroyed")))

(event EventTick
  (params (DeltaSeconds :type Float%20%28single-precision%29))
  (bind _springarm (Variables|Default|GetSpringArm))
  (bind _oxygenmaterial (Variables|Default|GetOxygenMaterial))
  (Utilities|FlowControl|Sequence
    (:then_0
      (Variables|/Script/Engine.SpringArmComponent|SetSocketOffset _springarm (Math|Vector|MakeVector (.X (Math|Vector|BreakVector (Variables|/Script/Engine.SpringArmComponent|GetSocketOffset _springarm))) (Math|Interpolation|FInterpTo (.Y (Math|Vector|BreakVector (Variables|/Script/Engine.SpringArmComponent|GetSocketOffset _springarm))) (Variables|Default|GetShoulderY) (Utilities|Time|GetWorldDeltaSeconds) 8.0) (.Z (Math|Vector|BreakVector (Variables|/Script/Engine.SpringArmComponent|GetSocketOffset _springarm))))))
    (:then_1
      (Variables|Default|SetCurrentOxygen (Math|Float|Clamp(Float) (- (Variables|Default|GetCurrentOxygen) (* (Variables|Default|GetOxygenDrainRate) DeltaSeconds)) 0.0 1e+02))
      (Rendering|Material|SetScalarParameterValue _oxygenmaterial "FillAmount" (/ (Variables|Default|GetCurrentOxygen) (Variables|Default|GetMaxOxygen)) :!class /Script/Engine.MaterialInstanceDynamic)
      (Rendering|Material|SetScalarParameterValue _oxygenmaterial "ColourBlend" (- 1.0 (/ (Variables|Default|GetCurrentOxygen) (Variables|Default|GetMaxOxygen))) :!class /Script/Engine.MaterialInstanceDynamic)
      (if (and (<= (Variables|Default|GetCurrentOxygen) 0.0) (not (Variables|Default|GetIsDead)))
        (Variables|Default|SetIsDead true)
        (Utilities|FlowControl|Delay 2.0)
        (Transformation|SetActorLocation (Variables|Default|GetLastCheckpointLocation) false false)
        ;[0.474 0.474 0.474 0.5] Sets the switches to match their state when last saved
        (bind _returnvalue (Actor|GetActorOfClass "/Game/Interaction/Actors/Oxygen_BP.Oxygen_BP_C"))
        (for (_array_element _array_index) (Variables|/Game/Interaction/Actors/Oxygen_BP.Oxygen_BP_C|GetSwitchList _returnvalue)
          (Variables|/Game/Interaction/Actors/Switch_BP.Switch_BP_C|SetisRedirected _array_element (Utilities|Array|Get(acopy) (Variables|/Game/Interaction/Actors/Oxygen_BP.Oxygen_BP_C|GetSwitchSaveList _returnvalue) _array_index))
          (Variables|Default|SetCurrentOxygen (Variables|Default|GetMaxOxygen))
          (Variables|Default|SetIsDead false))))
    (:then_2
      (if (Variables|Default|GetIsSprint)
        (bind _output_get (Variables|Default|SetCurrentStamina (Math|Float|Clamp(Float) (- (Variables|Default|GetCurrentStamina) (* (Variables|Default|GetStaminaConsume) (Utilities|Time|GetWorldDeltaSeconds))) 0.0 (Variables|Default|GetMaxStamina))))
        (Development|PrintString (Utilities|String|ToString(Float) _output_get) true true "(R=1.000000,G=0.687881,B=0.050316,A=1.000000)" 0.0)
        (else
          (Variables|Default|SetSprintingEndTime (+ (Variables|Default|GetSprintingEndTime) (Utilities|Time|GetWorldDeltaSeconds)))
          (if (>= (Variables|Default|GetSprintingEndTime) 4.0)
            (bind _output_get_2 (Variables|Default|SetCurrentStamina (Math|Float|Clamp(Float) (+ (Variables|Default|GetCurrentStamina) (* (Variables|Default|GetStaminaRecovery) (Utilities|Time|GetWorldDeltaSeconds))) 0.0 (Variables|Default|GetMaxStamina))))
            (Development|PrintString (Utilities|String|ToString(Float) _output_get_2) true true "(R=1.000000,G=0.099532,B=0.127229,A=1.000000)" 0.0)))))
    (:then_3
      (if (== (Variables|Default|GetCurrentStamina) 0.0)
        (Variables|/Script/Engine.CharacterMovementComponent|SetMaxWalkSpeed (Variables|Character|GetCharacterMovement) 5e+02)))))

(fn ConstructionScript)

(fn TextMenu
  (bind _foundwidgets (Widget|GetAllWidgetsOfClass "/Game/Text.Text_C" true))
  (if (Utilities|IsValid (Utilities|Array|Get(acopy) _foundwidgets))
    ;[0.599 0.599 0.599 0.5] Alternating Text Menu State
    (if (Variables|Default|GetIsTextActive)
      (Widget|RemovefromParent (Utilities|Array|Get(acopy) _foundwidgets))
      (Variables|Default|SetIsTextActive false)
      (else
        (UserInterface|Viewport|AddtoViewport (Utilities|Array|Get(acopy) _foundwidgets) 0)
        (Variables|Default|SetIsTextActive true)))
    (else
      ;[0.5104 0.5104 0.5104 0.5] Creating widget
      (bind _returnvalue (UserInterface|CreateWidget "/Game/Text.Text_C" (Game|GetPlayerController 0)))
      (UserInterface|Viewport|AddtoViewport _returnvalue 0)
      (Variables|Default|SetIsTextActive true))))
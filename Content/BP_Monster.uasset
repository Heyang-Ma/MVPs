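; BP_Monster is an AI enemy character, driven by AIC_Monster, that zeroes the oxygen of a BP_TestCharacterMerge overlapping its sphere.
; Stun halts movement, sets the blackboard's IsStunned flag and clears TargetActor, then a short timer calls RecoverFromStun to lift the flag and clear the target again.
; Tick wraps PatrolPointIndex to the first patrol point, while the index is not advanced here.
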(event OnComponentBeginOverlap(Sphere)
  (params (OverlappedComponent :type Primitive%20Component%20Object%20Reference) (OtherActor :type Actor%20Object%20Reference) (OtherComp :type Primitive%20Component%20Object%20Reference) (OtherBodyIndex :type Integer) (bFromSweep :type Boolean) (SweepResult :type Hit%20Result%20Structure%20%28by%20ref%29))
  (bind _asbp_test_character_merge (Utilities|Casting|CastToBP_TestCharacterMerge OtherActor))
  (Variables|/Game/BP_TestCharacterMerge.BP_TestCharacterMerge_C|SetCurrentOxygen _asbp_test_character_merge 0.0))

(event Custom|Stun
  (Development|PrintString "Monster stunned!")
  (bind _asaic_monster (Utilities|Casting|CastToAIC_Monster (Pawn|GetController)))
  (AI|Components|Blackboard|SetValueasBool (AI|GetBlackboard _asaic_monster) (Utilities|Name|MakeLiteralName "IsStunned") true)
  (Components|Movement|StopMovementImmediately (Variables|Character|GetCharacterMovement))
  (AI|Components|Blackboard|ClearValue (AI|GetBlackboard _asaic_monster) (Utilities|Name|MakeLiteralName "TargetActor"))
  (Utilities|Time|SetTimerbyEvent (delegate Custom|RecoverFromStun) 3.0))

(event Custom|RecoverFromStun
  (bind _asaic_monster (Utilities|Casting|CastToAIC_Monster (Pawn|GetController)))
  (AI|Components|Blackboard|SetValueasBool (AI|GetBlackboard _asaic_monster) (Utilities|Name|MakeLiteralName "IsStunned") false)
  (AI|Components|Blackboard|ClearValue (AI|GetBlackboard _asaic_monster) (Utilities|Name|MakeLiteralName "TargetActor"))
  (Development|PrintString "Monster recovered!"))

(event EventBeginPlay)

(event Collision|EventActorBeginOverlap
  (params (OtherActor :type Actor%20Object%20Reference)))

(event EventTick
  (params (DeltaSeconds :type Float%20%28single-precision%29))
  (if (== (Variables|Default|GetPatrol%20Point%20Index) (Utilities|Array|Length (Variables|Default|GetPatrolPoints)))
    (Variables|Default|SetPatrol%20Point%20Index 0)))

(fn ConstructionScript)